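; Debug actor that exposes player state and helper-function results during play.
; On BeginPlay it enables input, caches the BP_ThirdPersonCharacter and binds to its Health component's change event, with a handler that prints new health values.
; T prints the player's location, and F draws a one-frame visibility line trace forward from the player.
; Rotation and scale prints exist but are not wired up.
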(event `self.ReceiveBeginPlay`
  (`self.EnableInput` (`GameplayStatics.GetPlayerController` 0))
  (bind _asbp_third_person_character (cast `/Game/ThirdPerson/Blueprints/BP_ThirdPersonCharacter` (`PlayerCharacterHelpers.GetPlayerCharacterFromPlayerController` 0)))
  (set `self.PlayerCharacter` _asbp_third_person_character)
  (add `HealthComponent.OnHealthChanged` (`/Game/ThirdPerson/Blueprints/BP_ThirdPersonCharacter.Health` (`self.PlayerCharacter`)) (`|CreateDelegate` :!event `Event Player Health Changed`)))

(event `Key|T`
  (params (Key :type "Key Structure"))
  (:`Pressed`
    (`KismetSystemLibrary.PrintString` (`KismetStringLibrary.Conv_VectorToString` (`PlayerTransformHelpers.GetPlayerLocation` 0)))))

(event `Key|F`
  (params (Key :type "Key Structure"))
  (:`Pressed`
    (`KismetSystemLibrary.LineTraceSingle` :`Start` (`PlayerTransformHelpers.GetPlayerLocation` 0) :`End` (+ (* (`PlayerVectorHelpers.GetPlayerForwardVector` 0) 1000) (`PlayerTransformHelpers.GetPlayerLocation` 0)) :`TraceChannel` "TraceTypeQuery1" :`bTraceComplex` true :`DrawDebugType` "ForOneFrame")))

(event `Event Player Health Changed`
  (params (NewHealth :type Integer))
  (`KismetSystemLibrary.PrintString` (`KismetStringLibrary.Concat_StrStr` "PlayerDebug: " (`KismetStringLibrary.Conv_IntToString` NewHealth))))

(fn `UserConstructionScript`)